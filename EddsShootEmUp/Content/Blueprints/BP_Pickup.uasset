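; BP_Pickup is a collectible pickup actor that flies to a target and hands over its stats.
; CollectPickUp turns its ProjectileMovement into a homing projectile aimed at the target's root component and sets a high max speed.
; GetPickUpStats returns PickUpStats and also triggers DestroySelf, so reading the stats consumes the pickup.
; DestroySelf disables sphere collision and hides the actor, then destroys it after a short delay.
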(event Custom|DestroySelf
  (Collision|SetCollisionEnabled (Variables|Default|GetSphere) "NoCollision")
  (Rendering|SetActorHiddenInGame true)
  (Utilities|FlowControl|Delay 1.0)
  (Actor|DestroyActor))

(event EventCollectPickUp
  (params (HomingTarget :type Actor%20Object%20Reference))
  (bind _projectilemovement (Variables|Default|GetProjectileMovement))
  (Variables|/Script/Engine.ProjectileMovementComponent|SetHomingTargetComponent _projectilemovement (Variables|/Script/Engine.Actor|GetRootComponent HomingTarget))
  (Variables|/Script/Engine.ProjectileMovementComponent|SetbIsHomingProjectile _projectilemovement true)
  (Variables|/Script/Engine.ProjectileMovementComponent|SetMaxSpeed _projectilemovement 4e+03))

(fn ConstructionScript)

(fn GetPickUpStats
  (CallFunction|DestroySelf)
  (return (Variables|Default|GetPickUpStats)))