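; BP_EnemyB is an enemy that homes in on the player while firing bullets at a regular interval.
; On BeginPlay it runs the parent logic, starts a looping timer and sets the player pawn's root component as its ProjectileMovement homing target.
; Each timer tick spawns a BP_Projectile_EnemyBullet at the Arrow component's location and rotation.
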(event Custom|ShootBullet
  (bind _arrow (Variables|Default|GetArrow))
  (bind _returnvalue (Transformation|GetWorldTransform _arrow))
  ;[0.15 0.15 0.15 0.5] Spawn Enemy Bullet
  (Game|SpawnActorfromClass "/Game/Blueprints/BP_Projectile_EnemyBullet.BP_Projectile_EnemyBullet_C" (Math|Transform|MakeTransform (.location _returnvalue) (.rotation _returnvalue) "1.000000,1.000000,1.000000") "Undefined" "MultiplyWithRoot" 0 0))

(event EventBeginPlay
  ;[0.15 0.15 0.15 0.5] Begin Event + Time between bullets
  (|CallParentFunction)
  (Utilities|Time|SetTimerbyEvent (delegate Custom|ShootBullet) 2.0 true)
  (Variables|/Script/Engine.ProjectileMovementComponent|SetHomingTargetComponent (Variables|Default|GetProjectileMovement) (Variables|/Script/Engine.Actor|GetRootComponent (Game|Player|GetPlayerPawn 0))))

(fn ConstructionScript
  (|CallParentFunction))