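; Enemy spawner actor that continuously spawns BP_EnemyA along a line between two limit components.
; On BeginPlay it starts a looping one-second timer that calls SpawnEnemy.
; Each spawn picks a random point by lerping between the right and left limit world locations, using the left limit's rotation.
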(event Custom|SpawnEnemy
  (Game|SpawnActorfromClass "/Game/Blueprints/BP_EnemyA.BP_EnemyA_C" (Math|Transform|MakeTransform (Math|Vector|Lerp(Vector) (Transformation|GetWorldLocation (Variables|Default|GetRightSpawntLimit)) (Transformation|GetWorldLocation (Variables|Default|GetLeftSpawnLimit)) (Math|Random|RandomFloat)) (Transformation|GetWorldRotation (Variables|Default|GetLeftSpawnLimit)) "1.000000,1.000000,1.000000") "Undefined" "MultiplyWithRoot" 0 0))

(event EventBeginPlay
  (Utilities|Time|SetTimerbyEvent (delegate Custom|SpawnEnemy) 1.0 true))

(fn ConstructionScript)