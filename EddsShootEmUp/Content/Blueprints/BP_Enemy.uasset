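; BP_Enemy is an enemy actor that damages whatever it overlaps, dealing damage equal to its current Health.
; Incoming damage lowers Health, updates the WBP_EnemyHealthBar widget with the health fraction and spawns a BP_DamagePopup.
; A non-lethal hit plays a sound and shows a temporary overlay material on the mesh.
; At zero Health it plays a kill sound, spawns BP_Explosion and destroys itself.
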(event Custom|HitSequence
  (Audio|PlaySound2D "/Game/Audio/MS_Hit.MS_Hit" 0.5 1.0 0.0 0 0)
  (Rendering|Material|SetOverlayMaterial (Variables|Default|GetStaticMesh) "/Game/Materials/M_Overlay.M_Overlay" false 0 :!class /Script/Engine.MeshComponent)
  (Utilities|FlowControl|Delay 2.0)
  (Rendering|Material|SetOverlayMaterial (Variables|Default|GetStaticMesh) 0 false 0 :!class /Script/Engine.MeshComponent))

(event Custom|KillSequence
  (Audio|PlaySound2D "/Game/Audio/MS_Kill.MS_Kill" 0.5 1.0 0.0 0 0)
  (Game|SpawnActorfromClass "/Game/Particles/BP_Explosion.BP_Explosion_C" (Math|Transform|MakeTransform (Transformation|GetActorLocation) "0, 0, 0" "1.000000,1.000000,1.000000") "AlwaysSpawn" "MultiplyWithRoot" 0 0)
  (Actor|DestroyActor))

(event Collision|EventActorBeginOverlap
  (params (OtherActor :type Actor%20Object%20Reference))
  (Game|Damage|ApplyDamage OtherActor (Variables|Default|GetHealth) 0 0))

(event Game|Damage|EventAnyDamage
  (params (Damage :type Float%20%28single-precision%29) (DamageType :type Damage%20Type%20Object%20Reference) (InstigatedBy :type Controller%20Object%20Reference) (DamageCauser :type Actor%20Object%20Reference))
  (Variables|Default|SetHealth (Math|Float|Max(Float) (- (Variables|Default|GetHealth) Damage) 0.0))
  (Utilities|FlowControl|Sequence
    (:then_0
      ;[0.15 0.15 0.15 0.5] UI Update
      (bind _aswbp_enemy_health_bar (Utilities|Casting|CastToWBP_EnemyHealthBar (UserInterface|GetUserWidgetObject (Variables|Default|GetWidget))))
      (Default|SetHealth _aswbp_enemy_health_bar (Math|Float|SafeDivide (Variables|Default|GetHealth) (Variables|Default|GetMaxHealth))))
    (:then_1
      (Game|SpawnActorfromClass "/Game/UI/BP_DamagePopup.BP_DamagePopup_C" (Math|Transform|MakeTransform (Transformation|GetActorLocation) "0, 0, 0" "1.000000,1.000000,1.000000") "Undefined" "MultiplyWithRoot" 0 Damage 0))
    (:then_2
      (if (== (Variables|Default|GetHealth) 0.0)
        (CallFunction|KillSequence)
        (else
          (CallFunction|HitSequence))))))

(fn ConstructionScript)